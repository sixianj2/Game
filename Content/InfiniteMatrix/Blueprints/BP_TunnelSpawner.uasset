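; BP_TunnelSpawner builds the endless tunnel of the InfiniteMatrix level from chained BP_Tunnel segments.
; On BeginPlay it destroys existing tunnels and health-style BP_HPack pickups, then spawns an initial run starting at the player pawn, each next segment at the previous one's SpawnPoint.
; Each spawn stores a back-reference to the spawner, randomizes its wall, and places either a BP_HPack or BP_enemy at a random offset ahead.
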(event `self.ReceiveBeginPlay`
  (`self.SpawnInitialTunnels`))

(fn `SpawnInitialTunnels`
  (`|ExecutionSequence`
    (:`then_0`
      (bind _outactors (`GameplayStatics.GetAllActorsOfClass` "/Game/InfiniteMatrix/Blueprints/BP_Tunnel.BP_Tunnel_C"))
      (for _array_element _outactors
        (`self.K2_DestroyActor` _array_element)))
    (:`then_1`
      (bind _outactors_2 (`GameplayStatics.GetAllActorsOfClass` "/Game/InfiniteMatrix/Blueprints/BP_HPack.BP_HPack_C"))
      (for _array_element_2 _outactors_2
        (`self.K2_DestroyActor` _array_element_2)))
    (:`then_2`
      (for _ (range 26)
        (`/Engine/EditorBlueprintResources/StandardMacros.IsValid` (`self.NewestTunnel`)
          (:`Is Valid`
            (`self.SpawnTunnelAtSpawnPoint`))
          (:`Is Not Valid`
            (`self.SpawnTunnel` (`self.K2_GetActorLocation` (`GameplayStatics.GetPlayerPawn` 0)))))))))

(fn `SpawnTunnel`
  (params (SpawnLocation :type "Vector Structure"))
  (bind (_returnvalue_x _returnvalue_y _returnvalue_z) (break `IntVector` (`KismetMathLibrary.FTruncVector` SpawnLocation)))
  (bind _returnvalue (`KismetMathLibrary.Conv_IntToDouble` (+ _returnvalue_x (`KismetMathLibrary.RandomIntegerInRange` 500 800))))
  (bind _returnvalue_2 (`KismetMathLibrary.Conv_IntToDouble` (+ _returnvalue_y (`KismetMathLibrary.RandomIntegerInRange` -250 250))))
  (bind _returnvalue_3 (`KismetMathLibrary.Conv_IntToDouble` (+ _returnvalue_z (`KismetMathLibrary.RandomIntegerInRange` -250 250))))
  (bind _returnvalue_4 (`|SpawnActorFromClass` "/Game/InfiniteMatrix/Blueprints/BP_Tunnel.BP_Tunnel_C" (`KismetMathLibrary.MakeTransform` SpawnLocation) "Undefined" "OverrideRootScale" null null))
  (bind _output_get (set `self.NewestTunnel` _returnvalue_4))
  (set `/Game/InfiniteMatrix/Blueprints/BP_Tunnel.TunnelSpawner` self _output_get)
  (if (`KismetMathLibrary.RandomBoolWithWeight` 0.5)
    (`|SpawnActorFromClass` "/Game/InfiniteMatrix/Blueprints/BP_HPack.BP_HPack_C" (`KismetMathLibrary.MakeTransform` (`KismetMathLibrary.MakeVector` _returnvalue _returnvalue_2 _returnvalue_3)) "Undefined" "OverrideRootScale" null null)
    (else
      (`|SpawnActorFromClass` "/Game/InfiniteMatrix/Blueprints/BP_enemy.BP_enemy_C" (`KismetMathLibrary.MakeTransform` (`KismetMathLibrary.MakeVector` _returnvalue _returnvalue_2 _returnvalue_3)) "Undefined" "OverrideRootScale" null null)))
  (`/Game/InfiniteMatrix/Blueprints/BP_Tunnel.RandomizeWall` _output_get))

(fn `SpawnTunnelAtSpawnPoint`
  (`self.SpawnTunnel` (`SceneComponent.K2_GetComponentLocation` (`/Game/InfiniteMatrix/Blueprints/BP_Tunnel.SpawnPoint` (`self.NewestTunnel`)))))

(fn `UserConstructionScript`)